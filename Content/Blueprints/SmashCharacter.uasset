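; SmashCharacter is a character Blueprint that moves sideways along world Y for two local players sharing one keyboard.
; Each Tick switches on PlayerNumber and polls Player Controller 0 for that player's keys: J/L for player 0, A/D for player 1.
; Movement sets the actor location directly by a fixed step per frame, without sweep collision or delta-time scaling.
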(event EventTick
  (params (DeltaSeconds :type Float%20%28single-precision%29))
  (switch int (Variables|Default|GetPlayerNumber self)
    (:0
      ;[1 1 1] Player 0 Input
      (if (Game|Player|IsInputKeyDown (Game|GetPlayerController 0) "J")
        (Transformation|SetActorLocation (+ (Transformation|GetActorLocation) "0.000000,-2.000000,0.000000") false false)
        (elif (Game|Player|IsInputKeyDown (Game|GetPlayerController 0) "L")
          (Transformation|SetActorLocation (+ (Transformation|GetActorLocation) "0.000000,2.000000, 0") false false))))
    (:1
      ;[1 1 1] Player 1 Input
      (if (Game|Player|IsInputKeyDown (Game|GetPlayerController 0) "A")
        (Transformation|SetActorLocation (+ (Transformation|GetActorLocation) "0.000000,-2.000000, 0") false false)
        (elif (Game|Player|IsInputKeyDown (Game|GetPlayerController 0) "D")
          (Transformation|SetActorLocation (+ (Transformation|GetActorLocation) "0.000000,2.000000, 0") false false))))))

(fn ConstructionScript)